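; BP_Frog is the player frog in a Frogger game, hopping along X and Y through Enhanced Input.
; Each directional input turns the frog, plays a jump montage and runs a timeline that teleports it by Delta times JumpDistance each update.
; OnDeath disables input, spawns blood, flattens the frog and reloads the level after a delay.
; AddLily counts lily pads and pauses with a win screen at five; pause input opens a menu.
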(event Custom|OnDeath
  (Input|DisableInput (Game|GetPlayerController 0))
  (Niagara|SpawnSystematLocation "/Game/Frogger/Assets/VFX/Blood/NS_BloodSplat.NS_BloodSplat" (Transformation|GetActorLocation))
  (Transformation|SetActorScale3D "1.100000,1.100000,0.400000")
  (Utilities|FlowControl|Delay 2.0)
  (bind _returnvalue (Game|GetCurrentLevelName true))
  (Game|OpenLevel(byName) (Utilities|String|StringToName _returnvalue)))

(event Input|EnhancedActionEvents|EnhancedInputActionIA_Up
  (params (ActionValue :type Boolean) (ElapsedSeconds :type Float%20%28double-precision%29) (TriggeredSeconds :type Float%20%28double-precision%29) (InputAction :type Input%20Action%20Object%20Reference :default "/Game/Frogger/Input/IA_Up.IA_Up"))
  (bind _returnvalue (Transformation|GetActorLocation))
  (bind _returnvalue_2 (Transformation|GetActorLocation))
  ;[0 1 0.1206] Movement: Set frog rotation to be in direction of input and play jump animation; move frog forward by rate of jumping distance and maintain current rotation previously set
  (Transformation|SetActorRotation (Math|Rotator|FindLookatRotation _returnvalue_2 (+ _returnvalue_2 "1.000000,0.000000,0.000000")))
  (Animation|PlayAnimMontage "/Game/Frogger/Assets/Frog/animations/montages/7_metarig_jumpInPlace_Montage.7_metarig_jumpInPlace_Montage" 2.0 "None")
  (bind _delta (Timeline|Upward PlayFromStart)
    (:Update
      (Transformation|Teleport (Math|Vector|MakeVector (+ (.x _returnvalue) (* _delta (Variables|Default|GetJumpDistance))) (.y _returnvalue) (.z _returnvalue)) (Transformation|GetActorRotation)))))

(event Input|EnhancedActionEvents|EnhancedInputActionIA_Down
  (params (ActionValue :type Boolean) (ElapsedSeconds :type Float%20%28double-precision%29) (TriggeredSeconds :type Float%20%28double-precision%29) (InputAction :type Input%20Action%20Object%20Reference :default "/Game/Frogger/Input/IA_Down.IA_Down"))
  (bind _returnvalue (Transformation|GetActorLocation))
  (bind _returnvalue_2 (Transformation|GetActorLocation))
  ;[0 1 0.1206] Movement: Set frog rotation to be in direction of input and play jump animation; move frog forward by rate of jumping distance and maintain current rotation previously set
  (Transformation|SetActorRotation (Math|Rotator|FindLookatRotation _returnvalue_2 (+ _returnvalue_2 "-1.000000,0.000000,0.000000")))
  (Animation|PlayAnimMontage "/Game/Frogger/Assets/Frog/animations/montages/7_metarig_jumpInPlace_Montage.7_metarig_jumpInPlace_Montage" 2.0 "None")
  (bind _delta (Timeline|Timeline PlayFromStart)
    (:Update
      (Transformation|Teleport (Math|Vector|MakeVector (+ (.x _returnvalue) (* _delta (Variables|Default|GetJumpDistance))) (.y _returnvalue) (.z _returnvalue)) (Transformation|GetActorRotation)))))

(event Input|EnhancedActionEvents|EnhancedInputActionIA_Right
  (params (ActionValue :type Boolean) (ElapsedSeconds :type Float%20%28double-precision%29) (TriggeredSeconds :type Float%20%28double-precision%29) (InputAction :type Input%20Action%20Object%20Reference :default "/Game/Frogger/Input/IA_Right.IA_Right"))
  (bind _returnvalue (Transformation|GetActorLocation))
  (bind _returnvalue_2 (Transformation|GetActorLocation))
  ;[0 1 0.1206] Movement: Set frog rotation to be in direction of input and play jump animation; move frog forward by rate of jumping distance and maintain current rotation previously set
  (Transformation|SetActorRotation (Math|Rotator|FindLookatRotation _returnvalue (+ _returnvalue "0.000000,1.000000,0.000000")))
  (Animation|PlayAnimMontage "/Game/Frogger/Assets/Frog/animations/montages/7_metarig_jumpInPlace_Montage.7_metarig_jumpInPlace_Montage" 2.0 "None")
  (bind _delta (Timeline|Timeline_1 PlayFromStart)
    (:Update
      (Transformation|Teleport (Math|Vector|MakeVector (.x _returnvalue_2) (+ (.y _returnvalue_2) (* _delta (Variables|Default|GetJumpDistance))) (.z _returnvalue_2)) (Transformation|GetActorRotation)))))

(event Input|EnhancedActionEvents|EnhancedInputActionIA_Left
  (params (ActionValue :type Boolean) (ElapsedSeconds :type Float%20%28double-precision%29) (TriggeredSeconds :type Float%20%28double-precision%29) (InputAction :type Input%20Action%20Object%20Reference :default "/Game/Frogger/Input/IA_Left.IA_Left"))
  (bind _returnvalue (Transformation|GetActorLocation))
  (bind _returnvalue_2 (Transformation|GetActorLocation))
  ;[0 1 0.1206] Movement: Set frog rotation to be in direction of input and play jump animation; move frog forward by rate of jumping distance and maintain current rotation previously set
  (Transformation|SetActorRotation (Math|Rotator|FindLookatRotation _returnvalue_2 (+ _returnvalue_2 "0.000000,-1.000000,0.000000")))
  (Animation|PlayAnimMontage "/Game/Frogger/Assets/Frog/animations/montages/7_metarig_jumpInPlace_Montage.7_metarig_jumpInPlace_Montage" 2.0 "None")
  (bind _delta (Timeline|Timeline_0 PlayFromStart)
    (:Update
      (Transformation|Teleport (Math|Vector|MakeVector (.x _returnvalue) (+ (.y _returnvalue) (* _delta (Variables|Default|GetJumpDistance))) (.z _returnvalue)) (Transformation|GetActorRotation)))))

(event Input|EnhancedActionEvents|EnhancedInputActionIA_Pause
  (params (ActionValue :type Boolean) (ElapsedSeconds :type Float%20%28double-precision%29) (TriggeredSeconds :type Float%20%28double-precision%29) (InputAction :type Input%20Action%20Object%20Reference :default "/Game/Frogger/Input/IA_Pause.IA_Pause"))
  (Game|SetGamePaused true)
  (bind _returnvalue (UserInterface|CreateWidget "/Game/Frogger/UI/WBP_PauseMenu.WBP_PauseMenu_C"))
  (UserInterface|Viewport|AddtoViewport _returnvalue 0)
  (Variables|/Script/Engine.PlayerController|SetbShowMouseCursor (Game|GetPlayerController 0) true))

(event EventBeginPlay
  ;[0.3934 1 0.3188] Init input mapping
  (bind _asplayer_controller (Utilities|Casting|CastToPlayerController (Pawn|GetController)))
  (Input|AddMappingContext (PlayerController|LocalPlayerSubsystems|GetEnhancedInputLocalPlayerSubsystem _asplayer_controller) "/Game/Frogger/Input/IMC_FrogInputs.IMC_FrogInputs" 0 "(bIgnoreAllPressedKeysUntilRelease=True,bForceImmediately=False,bNotifyUserSettings=False)"))

(fn ConstructionScript)

(fn AddLily
  (bind _numlilypads (Variables|Default|GetNumLilyPads))
  (Math|Integer|IncrementInt _numlilypads
    (:%20%20
      (if (>= _numlilypads 5)
        (Game|SetGamePaused true)
        (bind _returnvalue (UserInterface|CreateWidget "/Game/Frogger/UI/WBP_WinScreen.WBP_WinScreen_C"))
        (UserInterface|Viewport|AddtoViewport _returnvalue 0)
        (Variables|/Script/Engine.PlayerController|SetbShowMouseCursor (Game|GetPlayerController 0) true)))))