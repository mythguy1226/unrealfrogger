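; BP_TeleporterSpawner is a Frogger actor that periodically spawns pairs of linked teleporters at random spots in the level.
; A timer set at BeginPlay and set again after each spawn paces SpawnTeleporters by SpawnInterval.
; FindNewEndpoints picks two random X/Y offsets within the Bounds box around the spawner, adding the actor's Z to its own location.
; Each new BP_Teleporter pair is cross-linked through LinkedTeleporter.
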(event Custom|Spawn%20Teleporters
  (bind (_endpoint1 _endpoint2) (CallFunction|FindNewEndpoints))
  (bind _returnvalue (Game|SpawnActorfromClass "/Game/Frogger/AI/BP_Teleporter.BP_Teleporter_C" (Math|Transform|MakeTransform _endpoint1) "Undefined" "MultiplyWithRoot" 0 0))
  (bind _returnvalue_2 (Game|SpawnActorfromClass "/Game/Frogger/AI/BP_Teleporter.BP_Teleporter_C" (Math|Transform|MakeTransform _endpoint2) "Undefined" "MultiplyWithRoot" 0 0))
  (bind _output_get (Variables|/Game/Frogger/AI/BP_Teleporter.BP_Teleporter_C|SetLinkedTeleporter _returnvalue_2 _returnvalue))
  (Variables|/Game/Frogger/AI/BP_Teleporter.BP_Teleporter_C|SetLinkedTeleporter _output_get _returnvalue_2)
  (Utilities|Time|SetTimerbyEvent (EventDispatchers|CreateEvent :!event Custom|Spawn%20Teleporters) (Variables|Default|GetSpawnInterval)))

(event EventBeginPlay
  (Utilities|Time|SetTimerbyEvent (EventDispatchers|CreateEvent :!event Custom|Spawn%20Teleporters) (Variables|Default|GetSpawnInterval)))

(fn ConstructionScript)

(fn FindNewEndpoints
  (bind _returnvalue (Transformation|GetActorLocation))
  (bind _returnvalue_2 (Transformation|GetActorLocation))
  (bind _bounds (Variables|Default|GetBounds))
  (bind _bounds_2 (Variables|Default|GetBounds))
  (bind _returnvalue_3 (Components|Box|GetScaledBoxExtent _bounds))
  (bind _returnvalue_4 (Components|Box|GetScaledBoxExtent _bounds_2))
  ;[1 1 1] Calculate two random endpoints in the level
  (return (+ _returnvalue_2 (Math|Vector|MakeVector (Math|Random|RandomFloatinRange (* (.x _returnvalue_4) -1.0) (.x _returnvalue_4)) (Math|Random|RandomFloatinRange (* (.y _returnvalue_4) -1.0) (.y _returnvalue_4)) (.z _returnvalue))) (+ _returnvalue_2 (Math|Vector|MakeVector (Math|Random|RandomFloatinRange (* (.x _returnvalue_3) -1.0) (.x _returnvalue_3)) (Math|Random|RandomFloatinRange (* (.y _returnvalue_3) -1.0) (.y _returnvalue_3)) (.z _returnvalue)))))