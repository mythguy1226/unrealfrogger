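; Frogger turtle platform that periodically disappears and reappears, warning of each dive with a color change.
; A timer starts the flip after TimeToFlip, and a timeline drives the Color parameter on a dynamic material instance.
; When the timeline finishes, the actor is hidden for TimeFlipped, then shown with its color reset and the timer re-armed.
; Only visibility is toggled, with no explicit collision change.
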(event Custom|Flip
  (bind _colorswap (Timeline|ColorChange PlayFromStart)
    (:Update
      (Rendering|Material|SetVectorParameterValue (Variables|Default|GetMaterial) "Color" _colorswap :!class /Script/Engine.MaterialInstanceDynamic))
    (:Finished
      (Rendering|SetActorHiddenInGame true)
      (Utilities|FlowControl|Delay (Variables|Default|GetTimeFlipped))
      (Rendering|SetActorHiddenInGame false)
      (Rendering|Material|SetVectorParameterValue (Variables|Default|GetMaterial) "Color" "(R=0.349020,G=0.054902,B=0.000000,A=1.000000)" :!class /Script/Engine.MaterialInstanceDynamic)
      (Utilities|Time|SetTimerbyEvent (EventDispatchers|CreateEvent :!event Custom|Flip) (Variables|Default|GetTimeToFlip)))))

(event EventBeginPlay
  (bind _returnvalue (Rendering|Material|CreateDynamicMaterialInstance "/Game/Frogger/Materials/M_TurtlePlatform.M_TurtlePlatform" "None" "None" :!class /Script/Engine.KismetMaterialLibrary))
  (Variables|Default|SetMaterial _returnvalue)
  (Utilities|Time|SetTimerbyEvent (EventDispatchers|CreateEvent :!event Custom|Flip) (Variables|Default|GetTimeToFlip)))

(event EventTick
  (params (DeltaSeconds :type Float%20%28single-precision%29))
  (|CallParentFunction DeltaSeconds) ; This node is disabled and will not be called.\nDrag off pins to build functionality.
)

(fn ConstructionScript
  (|CallParentFunction))