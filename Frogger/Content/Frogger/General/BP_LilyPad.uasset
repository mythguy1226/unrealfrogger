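; BP_LilyPad is a goal lily pad in the Frogger game that records progress when the player's frog reaches it.
; On box overlap with BP_Frog, it calls AddLily on the frog to advance the count.
; It then adds a static mesh frog at the PerchPoint, rotated and scaled down, and moves the player back to the PlayerStart location.
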(event OnComponentBeginOverlap(Box)
  (params (OverlappedComponent :type Primitive%20Component%20Object%20Reference) (OtherActor :type Actor%20Object%20Reference) (OtherComp :type Primitive%20Component%20Object%20Reference) (OtherBodyIndex :type Integer) (bFromSweep :type Boolean) (SweepResult :type Hit%20Result%20Structure%20%28by%20ref%29))
  ;[1 1 1] When the player collides with the lily pad, add to counter for progression, spawn a static mesh of a frog on top of the pad, and move player back to start
  (bind _asbp_frog (Utilities|Casting|CastToBP_Frog OtherActor))
  (Default|AddLily _asbp_frog)
  (bind _returnvalue (AddComponent|AddStaticMeshComponent false (Math|Transform|MakeRelativeTransform (Math|Transform|MakeTransform (Variables|/Script/Engine.SceneComponent|GetRelativeLocation (Variables|Default|GetPerchPoint)) (Math|Vector|RotatorfromAxisandAngle "0.000000,0.000000,1.000000" 9e+01) "0.400000,0.200000,0.200000") (Math|Transform|MakeTransform (Variables|/Script/Engine.SceneComponent|GetRelativeLocation (Variables|Default|GetStaticMesh))))))
  (Components|StaticMesh|SetStaticMesh _returnvalue "/Game/Frogger/Assets/Frog/SM_Frog.SM_Frog")
  (bind _returnvalue_2 (Actor|GetActorOfClass "/Script/Engine.PlayerStart"))
  (Transformation|SetActorLocation _asbp_frog (Transformation|GetActorLocation _returnvalue_2) false false))

(fn ConstructionScript)